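; Base floor tile for a three-lane endless runner that spawns random obstacles on BeginPlay.
; SpawnObstacles rolls pipe or stone obstacles at lane markers, rolling the middle lane only after a left Obstacle_Pipe and the right only after a middle one.
; When the character overlaps its Box, the tile asks ThirdPersonGameMode for another tile, adds and prints multiplied points, raises clamped walk speed, then destroys itself after a short delay.
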(event OnComponentBeginOverlap(Box)
  (params (OverlappedComponent :type Primitive%20Component%20Object%20Reference) (OtherActor :type Actor%20Object%20Reference) (OtherComp :type Primitive%20Component%20Object%20Reference) (OtherBodyIndex :type Integer) (bFromSweep :type Boolean) (SweepResult :type Hit%20Result%20Structure%20%28by%20ref%29))
  (Utilities|Casting|CastToThirdPersonCharacter OtherActor)
  (bind _asthird_person_game_mode (Utilities|Casting|CastToThirdPersonGameMode (Game|GetGameMode)))
  (Default|SpawnTile _asthird_person_game_mode)
  (bind _asthird_person_game_mode_2 (Utilities|Casting|CastToThirdPersonGameMode (Game|GetGameMode)))
  (bind _output_get (Variables|/Game/ThirdPersonBP/Blueprints/ThirdPersonGameMode.ThirdPersonGameMode_C|SetCurrentPoints _asthird_person_game_mode_2 (+ (* 1 (Variables|/Game/ThirdPersonBP/Blueprints/ThirdPersonGameMode.ThirdPersonGameMode_C|GetPointsMultiplayer _asthird_person_game_mode_2)) (Variables|/Game/ThirdPersonBP/Blueprints/ThirdPersonGameMode.ThirdPersonGameMode_C|GetCurrentPoints _asthird_person_game_mode_2))))
  (Development|PrintString (Utilities|String|ToString(Integer) _output_get))
  (bind _asthird_person_character (Utilities|Casting|CastToThirdPersonCharacter (Game|GetPlayerCharacter 0)))
  (Variables|/Script/Engine.CharacterMovementComponent|SetMaxWalkSpeed (Variables|/Script/Engine.Character|GetCharacterMovement _asthird_person_character) (Math|Float|Clamp(Float) (* (Variables|/Script/Engine.CharacterMovementComponent|GetMaxWalkSpeed (Variables|/Script/Engine.Character|GetCharacterMovement _asthird_person_character)) 1.5) 6e+02 1.2e+03))
  (Utilities|FlowControl|Delay 0.4)
  (Actor|DestroyActor))

(event EventBeginPlay
  (CallFunction|SpawnObstacles))

(event Collision|EventActorBeginOverlap
  (params (OtherActor :type Actor%20Object%20Reference)))

(event EventTick
  (params (DeltaSeconds :type Float%20%28single-precision%29)))

(fn ConstructionScript)

(fn SpawnObstacles
  (bind _leftlane (Variables|Default|GetLeftLane))
  (bind _middlelane (Variables|Default|GetMiddleLane))
  (bind _rightlane (Variables|Default|GetRightLane))
  (bind _returnvalue (Transformation|GetWorldTransform _leftlane))
  (bind _returnvalue_2 (Transformation|GetWorldTransform _middlelane))
  (bind _returnvalue_3 (Transformation|GetWorldTransform _rightlane))
  ;[1 1 1] Left line
  (switch int (Math|Random|RandomIntegerinRange 0 6)
    (:1
      (Game|SpawnActorfromClass "/Game/RunnerPersonFiles/Blueprints/Obstacle_Pipe.Obstacle_Pipe_C" _returnvalue "Undefined" 0 0)
      ;[1 1 1] Middle line
      (switch int (Math|Random|RandomIntegerinRange 0 6)
        (:1
          (Game|SpawnActorfromClass "/Game/RunnerPersonFiles/Blueprints/Obstacle_Pipe.Obstacle_Pipe_C" _returnvalue_2 "Undefined" 0 0)
          ;[1 1 1] Right line
          (switch int (Math|Random|RandomIntegerinRange 0 2)
            (:1
              (Game|SpawnActorfromClass "/Game/RunnerPersonFiles/Blueprints/Obstacle_Pipe.Obstacle_Pipe_C" _returnvalue_3 "Undefined" 0 0))
            (:2
              (Game|SpawnActorfromClass "/Game/RunnerPersonFiles/Blueprints/Obstacle_Pipe2.Obstacle_Pipe2_C" _returnvalue_3 "Undefined" 0 0))))
        (:2
          (Game|SpawnActorfromClass "/Game/RunnerPersonFiles/Blueprints/Obstacle_Pipe2.Obstacle_Pipe2_C" _returnvalue_2 "Undefined" 0 0))
        (:3
          (Game|SpawnActorfromClass "/Game/RunnerPersonFiles/Blueprints/Obstacle_stone.Obstacle_stone_C" _returnvalue_2 "Undefined" 0 0))))
    (:2
      (Game|SpawnActorfromClass "/Game/RunnerPersonFiles/Blueprints/Obstacle_Pipe2.Obstacle_Pipe2_C" _returnvalue "Undefined" 0 0))
    (:3
      (Game|SpawnActorfromClass "/Game/RunnerPersonFiles/Blueprints/Obstacle_stone.Obstacle_stone_C" _returnvalue "Undefined" 0 0))))